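; Playable "Bru" character with a flipbook sprite that can be swapped into by clicking it, destroying the body left behind.
; While possessed, Tick line-traces to pawns gathered by a collider and outlines visible ones through InteractiveObjectsInterface using custom depth.
; Clicking an outlined instance possesses it, and Unpossessed destroys the actor.
; Input drives camera-boom-relative movement, jump and pause, while movement state and input set flipbook, play rate and left/right facing.
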(event `InputAction|Jump`
  (params (Key :type "Key Structure"))
  (:`Pressed`
    (`self.Jump`)
    (`PaperFlipbookComponent.SetFlipbook` (`self.da`) "/Game/Mannequin/JumpAnim/pcadr10.pcadr10")
    (set `self.Jumping` true)))

(event `InputAction|Pause`
  (params (Key :type "Key Structure"))
  (:`Pressed`
    (`GameplayStatics.SetGamePaused` (not (`GameplayStatics.IsGamePaused`)))))

(event `self.ReceiveBeginPlay`)

(event `self.ReceivePossessed`
  (params (NewController :type "Controller Object Reference"))
  (bind _returnvalue (`GameplayStatics.GetPlayerController` 0))
  (set `PlayerController.bShowMouseCursor` true _returnvalue)
  (set `PlayerController.bEnableClickEvents` true _returnvalue))

(event `self.ReceiveTick`
  (params (DeltaSeconds :type "Float (single-precision)"))
  (bind _returnvalue (`GameplayStatics.GetPlayerPawn` 0))
  (bind _da (`self.da`))
  (for _array_element (`self.OverlappingActors`)
    (if (and (!= _array_element _returnvalue) (== _returnvalue self))
      (bind _outhit (`KismetSystemLibrary.LineTraceSingle` (`self.K2_GetActorLocation`) (`self.K2_GetActorLocation` _array_element) "TraceTypeQuery1"))
      (bind _asinteractive_objects_interface (cast `/Game/Blueprint/InteractiveObjectsInterface` _array_element))
      (`self.ChangeOutline` _asinteractive_objects_interface (== (`.HitActor` (`GameplayStatics.BreakHitResult` _outhit)) _array_element))))
  (switch `EMovementMode` (`CharacterMovementComponent.MovementMode` (`self.CharacterMovement`))
    (:`MOVE_Walking`
      (`PaperFlipbookComponent.SetFlipbook` _da "/Game/Mannequin/cadr10.cadr10"))
    (:`MOVE_Falling`
      (`PaperFlipbookComponent.SetPlayRate` _da 1.0)
      (if (`self.Jumping`)
        (`KismetSystemLibrary.Delay` 0.5)
        (set `self.Jumping` false)
        (else
          (`PaperFlipbookComponent.SetFlipbook` _da "/Game/Mannequin/JumpAnim/Falling.Falling"))))))

(event `self.ColliderOfObject.OnComponentBeginOverlap`
  (params (OverlappedComponent :type "PrimitiveComponent Object Reference") (OtherActor :type "Actor Object Reference") (OtherComp :type "PrimitiveComponent Object Reference") (OtherBodyIndex :type Integer) (bFromSweep :type Boolean) (SweepResult :type "HitResult Structure (by ref)"))
  (bind (_aspawn _bsuccess) (cast `Pawn` OtherActor :!pure true))
  (if (and (!= OtherActor self) _bsuccess)
    (`KismetArrayLibrary.Array_AddUnique` (`self.OverlappingActors`) _aspawn)))

(event `self.ColliderOfObject.OnComponentEndOverlap`
  (params (OverlappedComponent :type "PrimitiveComponent Object Reference") (OtherActor :type "Actor Object Reference") (OtherComp :type "PrimitiveComponent Object Reference") (OtherBodyIndex :type Integer))
  (bind _asinteractive_objects_interface (cast `/Game/Blueprint/InteractiveObjectsInterface` OtherActor))
  (`self.ChangeOutline` _asinteractive_objects_interface false)
  (bind _aspawn (cast `Pawn` OtherActor))
  (`KismetArrayLibrary.Array_RemoveItem` (`self.OverlappingActors`) _aspawn))

(event `self.ChangeOutline`
  (params (isInRange :type Boolean))
  (`PrimitiveComponent.SetRenderCustomDepth` (`self.Mesh`) isInRange)
  (set `self.isOutline` isInRange))

(event `self.ReceiveActorOnClicked`
  (params (ButtonPressed :type "Key Structure"))
  (if (`self.isOutline`)
    (`Controller.Possess` (`GameplayStatics.GetPlayerController` 0) self)
    (`self.ChangeOutline` false)
    (set `self.isOutline` false)))

(event `InputAxis|MoveForward`
  (params (AxisValue :type "Float (single-precision)"))
  (if (!= AxisValue 0.0)
    (`self.AddMovementInput` (`SceneComponent.GetForwardVector` (`self.CameraBoom`)) AxisValue)
    (if (`CharacterMovementComponent.IsWalking` (`self.CharacterMovement`))
      (`PaperFlipbookComponent.SetPlayRate` (`self.da`) 1.0))))

(event `self.ReceiveUnpossessed`
  (params (OldController :type "Controller Object Reference"))
  (`self.K2_DestroyActor`))

(event `InputAxis|MoveRight`
  (params (AxisValue :type "Float (single-precision)"))
  (bind _da (`self.da`))
  (if (!= AxisValue 0.0)
    (`self.AddMovementInput` (`SceneComponent.GetRightVector` (`self.CameraBoom`)) AxisValue)
    (`PaperFlipbookComponent.SetPlayRate` (`self.da`) 1.0)
    (if (> AxisValue 0.0)
      (`SceneComponent.K2_SetWorldRotation` _da (struct :`Yaw` -90.0) false false)
      (else
        (`SceneComponent.K2_SetWorldRotation` _da (struct :`Yaw` 90.0) false false)))
    (elif (`CharacterMovementComponent.IsWalking` (`self.CharacterMovement`))
      (`PaperFlipbookComponent.SetPlayRate` (`self.da`) 0.0))))

(fn `UserConstructionScript`)