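; Floor button that switches off its linked firewall while a BP_CubeFirewall cube rests on it.
; A cube's capsule entering the collision sets the pressed state, calls ChangeActive on the firewall and plays a timeline that moves the button mesh along Z.
; When a cube leaves, it checks for other overlapping cubes and only reactivates the firewall and reverses the timeline if none remain.
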(event `self.ButtonCollision.OnComponentBeginOverlap`
  (params (OverlappedComponent :type "PrimitiveComponent Object Reference") (OtherActor :type "Actor Object Reference") (OtherComp :type "PrimitiveComponent Object Reference") (OtherBodyIndex :type Integer) (bFromSweep :type Boolean) (SweepResult :type "HitResult Structure (by ref)"))
  (cast `CapsuleComponent` OtherComp)
  (cast `/Game/Blueprint/NeededBP/BP_CubeFirewall` OtherActor)
  (bind _output_get (set `self.isPressed` true))
  (`/Game/Blueprint/NeededBP/Firewall.ChangeActive` (`self.LinkedFirewall`) (not _output_get))
  (bind (_direction _newtrack_0) (`Timeline|Timeline_0` :!label _label)
    (:`Update`
      (`SceneComponent.K2_SetRelativeLocation` (`self.ButtonMesh`) (`KismetMathLibrary.MakeVector` 0.0 0.0 _newtrack_0) false false))))

(event `self.ButtonCollision.OnComponentEndOverlap`
  (params (OverlappedComponent :type "PrimitiveComponent Object Reference") (OtherActor :type "Actor Object Reference") (OtherComp :type "PrimitiveComponent Object Reference") (OtherBodyIndex :type Integer))
  (cast `/Game/Blueprint/NeededBP/BP_CubeFirewall` OtherActor)
  (set `self.MassOk` false)
  (for _ (`PrimitiveComponent.GetOverlappingActors` (`self.ButtonCollision`) "/Game/Blueprint/NeededBP/BP_CubeFirewall.BP_CubeFirewall_C")
    (set `self.MassOk` true))
  (if (not (`self.MassOk`))
    (bind _output_get (set `self.isPressed` false))
    (`/Game/Blueprint/NeededBP/Firewall.ChangeActive` (`self.LinkedFirewall`) (not _output_get))
    (goto _label :!via `Reverse`)))

(fn `UserConstructionScript`
  (`parent.UserConstructionScript`))