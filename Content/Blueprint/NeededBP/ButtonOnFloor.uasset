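; A floor button that is pressed while a BP_ButtonInteractiveCharacter stands on it and notifies a linked actor of its state.
; Overlap by such a character's static mesh component sets it pressed, calls ButtonChangePressed on LinkedActor and plays a timeline lowering or moving the button mesh along Z.
; On end overlap, it releases and reverses the timeline only when no interactive characters remain in the collision.
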(event `self.ButtonCollision.OnComponentBeginOverlap`
  (params (OverlappedComponent :type "PrimitiveComponent Object Reference") (OtherActor :type "Actor Object Reference") (OtherComp :type "PrimitiveComponent Object Reference") (OtherBodyIndex :type Integer) (bFromSweep :type Boolean) (SweepResult :type "HitResult Structure (by ref)"))
  (cast `StaticMeshComponent` OtherComp)
  (cast `/Game/Blueprint/NeededBP/BP_ButtonInteractiveCharacter` OtherActor)
  (bind _output_get (set `self.isPressed` true))
  (`/Game/Blueprint/NeededBP/LinkedWithTheButton.ButtonChangePressed` (`self.LinkedActor`) _output_get)
  (bind (_direction _newtrack_0) (`Timeline|Press` :!label _label)
    (:`Update`
      (`SceneComponent.K2_SetRelativeLocation` (`self.ButtonMesh`) (`KismetMathLibrary.MakeVector` 0.0 0.0 _newtrack_0) false false))))

(event `self.ButtonCollision.OnComponentEndOverlap`
  (params (OverlappedComponent :type "PrimitiveComponent Object Reference") (OtherActor :type "Actor Object Reference") (OtherComp :type "PrimitiveComponent Object Reference") (OtherBodyIndex :type Integer))
  (cast `/Game/Blueprint/NeededBP/BP_ButtonInteractiveCharacter` OtherActor)
  (set `self.MassOk` false)
  (for _ (`PrimitiveComponent.GetOverlappingActors` (`self.ButtonCollision`) "/Game/Blueprint/NeededBP/BP_ButtonInteractiveCharacter.BP_ButtonInteractiveCharacter_C")
    (set `self.MassOk` true))
  (if (not (`self.MassOk`))
    (bind _output_get (set `self.isPressed` false))
    (`/Game/Blueprint/NeededBP/LinkedWithTheButton.ButtonChangePressed` (`self.LinkedActor`) _output_get)
    (goto _label :!via `Reverse`)))

(fn `UserConstructionScript`)