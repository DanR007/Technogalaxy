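; BackZoneTemp is a moving trigger zone that loads the Tempogame level when it touches the player character.
; Tick slides the actor at constant speed opposite its right vector, without sweep.
; Box overlap opens the level only if the other actor is player character 0 and the touched component is a static mesh or capsule.
; BeginPlay stores the owner in ActorOwn, which is not used afterward.
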(event `self.ReceiveBeginPlay`
  (`parent.ReceiveBeginPlay`)
  (set `self.actorOwn` (`self.GetOwner`)))

(event `self.ReceiveTick`
  (params (DeltaSeconds :type "Float (single-precision)"))
  (`parent.ReceiveTick` DeltaSeconds)
  (`self.K2_AddActorWorldOffset` (* (`self.GetActorRightVector`) (* DeltaSeconds -800.0))))

(event `self.Box.OnComponentBeginOverlap`
  (params (OverlappedComponent :type "PrimitiveComponent Object Reference") (OtherActor :type "Actor Object Reference") (OtherComp :type "PrimitiveComponent Object Reference") (OtherBodyIndex :type Integer) (bFromSweep :type Boolean) (SweepResult :type "HitResult Structure (by ref)"))
  (if (and (== OtherActor (`GameplayStatics.GetPlayerCharacter` 0)) (or (`.bSuccess` (cast `StaticMeshComponent` OtherComp :!pure true)) (`.bSuccess` (cast `CapsuleComponent` OtherComp :!pure true))))
    (`GameplayStatics.OpenLevelBySoftObjectPtr` "/Game/Levels/Tempogame.Tempogame")))

(fn `UserConstructionScript`
  (`parent.UserConstructionScript`))