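; BP_ButtonInteractiveCharacter is a character the player can take control of by clicking it and later leave.
; A capsule click runs a visibility trace to the current player character and possesses this character if that player is the hit actor.
; Pressing Crouch or overlapping a Barrier spawns a new BP_BruCharacter just ahead and hands possession to it, without destroying this character.
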(event `self.CapsuleComponent.OnComponentBeginOverlap`
  (params (OverlappedComponent :type "PrimitiveComponent Object Reference") (OtherActor :type "Actor Object Reference") (OtherComp :type "PrimitiveComponent Object Reference") (OtherBodyIndex :type Integer) (bFromSweep :type Boolean) (SweepResult :type "HitResult Structure (by ref)"))
  (bind (_returnvalue_location _returnvalue_rotation _returnvalue_scale) (`KismetMathLibrary.BreakTransform` (`self.GetTransform`)))
  (cast `/Game/Blueprint/NeededBP/Barrier` OtherActor)
  (bind _returnvalue (`|SpawnActorFromClass` "/Game/Blueprint/NeededBP/BP_BruCharacter.BP_BruCharacter_C" (`KismetMathLibrary.MakeTransform` (+ _returnvalue_location (* (`self.GetActorForwardVector`) 20.0)) _returnvalue_rotation _returnvalue_scale) "AdjustIfPossibleButAlwaysSpawn" "OverrideRootScale" null null :!label _label))
  (`Controller.Possess` (`GameplayStatics.GetPlayerController` 0) _returnvalue))

(event `InputAction|Crouch`
  (params (Key :type "Key Structure"))
  (:`Pressed`
    (goto _label)))

(event `self.CapsuleComponent.OnClicked`
  (params (TouchedComponent :type "PrimitiveComponent Object Reference") (ButtonPressed :type "Key Structure"))
  (bind _returnvalue (`GameplayStatics.GetPlayerCharacter` 0))
  (bind _outhit (`KismetSystemLibrary.LineTraceSingle` (`self.K2_GetActorLocation`) (`self.K2_GetActorLocation` _returnvalue) "TraceTypeQuery1"))
  (if (== (`.HitActor` (`GameplayStatics.BreakHitResult` _outhit)) _returnvalue)
    (`Controller.Possess` (`GameplayStatics.GetPlayerController` 0) self)))

(fn `UserConstructionScript`
  (`parent.UserConstructionScript`))