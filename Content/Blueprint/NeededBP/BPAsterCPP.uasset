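; Asteroid actor for a space shooter that drifts opposite its forward vector at a set speed and shows a random flipbook picked on BeginPlay.
; Overlapping the SpaceShuttle with its sphere calls the shuttle's collision handler, then explodes and destroys the asteroid.
; DamageApply reduces HP and, on a lethal hit, adds score through the ManagerCPP found at BeginPlay before the same explosion and destruction.
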(event `self.ReceiveBeginPlay`
  (bind _output_get (set `self.Images` (`|MakeArray` "/Game/Mannequin/SpaceShooter/aster3.aster3" "/Game/Mannequin/SpaceShooter/aster5.aster5" "/Game/Mannequin/SpaceShooter/aster6.aster6" "/Game/Mannequin/SpaceShooter/pkzpr2.pkzpr2" "/Game/Mannequin/SpaceShooter/pkzpr8.pkzpr8" "/Game/Mannequin/SpaceShooter/pkzpr9.pkzpr9" :!type "PaperFlipbook Object Reference")))
  (`PaperFlipbookComponent.SetFlipbook` (`self.PaperFlipbook`) (`|GetArrayItem` _output_get (`KismetMathLibrary.RandomIntegerInRange` 0 (- (`KismetArrayLibrary.Array_Length` _output_get) 1))))
  (bind _returnvalue (`GameplayStatics.GetActorOfClass` "/Script/ROBOTERRAbackstory.ManagerCPP"))
  (set `self.ManagerCPP` _returnvalue))

(event `self.ReceiveTick`
  (params (DeltaSeconds :type "Float (single-precision)"))
  (`self.K2_AddActorWorldOffset` (* (`self.GetActorForwardVector`) (* (`self.speed`) -1.0))))

(event `self.Sphere.OnComponentBeginOverlap`
  (params (OverlappedComponent :type "PrimitiveComponent Object Reference") (OtherActor :type "Actor Object Reference") (OtherComp :type "PrimitiveComponent Object Reference") (OtherBodyIndex :type Integer) (bFromSweep :type Boolean) (SweepResult :type "HitResult Structure (by ref)"))
  (bind _asspace_shuttle (cast `/Game/Blueprint/NeededBP/SpaceShuttle` OtherActor))
  (`/Game/Blueprint/NeededBP/SpaceShuttle.CollisionWithAsteroid` _asspace_shuttle)
  (`GameplayStatics.SpawnEmitterAtLocation` "/Game/Meshes/Particles/P_Explosion.P_Explosion" (`self.K2_GetActorLocation`))
  (`GameplayStatics.PlaySound2D` "/Game/Meshes/Audio/Explosion01.Explosion01" 1.0 1.0 0.0 null null)
  (`self.K2_DestroyActor`))

(fn `DamageApply`
  (params (NewParam :type Integer))
  (if (<= (- (`self.HP`) NewParam) 0)
    (`ManagerCPP.AddScore` (`self.ManagerCPP`) (`self.ScoreAdd`))
    (`GameplayStatics.SpawnEmitterAtLocation` "/Game/Meshes/Particles/P_Explosion.P_Explosion" (`self.K2_GetActorLocation`))
    (`GameplayStatics.PlaySound2D` "/Game/Meshes/Audio/Explosion01.Explosion01" 1.0 1.0 0.0 null null)
    (`self.K2_DestroyActor`)
    (else
      (set `self.HP` (- (`self.HP`) NewParam)))))

(fn `UserConstructionScript`)