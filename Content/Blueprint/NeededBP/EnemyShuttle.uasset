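; EnemyShuttle is an enemy ship that moves backward along its forward vector every tick at its Speed.
; On BeginPlay it finds ManagerCPP and, above a level multiplier threshold, gains extra HP and speed.
; Either collision box overlapping the player's SpaceShuttle calls CollisionWithAsteroid on it, then the enemy explodes and is destroyed.
; DamageApply reduces HP, and a lethal hit adds score through the manager before the same explosion and destruction.
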(event `self.ReceiveBeginPlay`
  (bind _levelmultiplier (`ManagerCPP.levelMultiplier` (`self.ManagerCPP`)))
  (bind _returnvalue (`GameplayStatics.GetActorOfClass` "/Script/Bru.ManagerCPP"))
  (set `self.ManagerCPP` _returnvalue)
  (if (> _levelmultiplier 4)
    (set `self.HP` (+ (`self.HP`) (- _levelmultiplier 3)))
    (set `self.Speed` (+ (`self.Speed`) (/ _levelmultiplier 1)))))

(event `self.ReceiveTick`
  (params (DeltaSeconds :type "Float (single-precision)"))
  (`self.K2_AddActorWorldOffset` (* (`self.GetActorForwardVector`) (* (`self.Speed`) -1.0))))

(event `self.Box.OnComponentBeginOverlap`
  (params (OverlappedComponent :type "PrimitiveComponent Object Reference") (OtherActor :type "Actor Object Reference") (OtherComp :type "PrimitiveComponent Object Reference") (OtherBodyIndex :type Integer) (bFromSweep :type Boolean) (SweepResult :type "HitResult Structure (by ref)"))
  (bind _asspace_shuttle (cast `/Game/Blueprint/NeededBP/SpaceShuttle` OtherActor))
  (`/Game/Blueprint/NeededBP/SpaceShuttle.CollisionWithAsteroid` _asspace_shuttle)
  (`GameplayStatics.SpawnEmitterAtLocation` "/Game/StarterContent/Particles/P_Explosion.P_Explosion" (`self.K2_GetActorLocation`) :!label _label)
  (`self.K2_DestroyActor`))

(event `self.Box1.OnComponentBeginOverlap`
  (params (OverlappedComponent :type "PrimitiveComponent Object Reference") (OtherActor :type "Actor Object Reference") (OtherComp :type "PrimitiveComponent Object Reference") (OtherBodyIndex :type Integer) (bFromSweep :type Boolean) (SweepResult :type "HitResult Structure (by ref)"))
  (bind _asspace_shuttle (cast `/Game/Blueprint/NeededBP/SpaceShuttle` OtherActor))
  (`/Game/Blueprint/NeededBP/SpaceShuttle.CollisionWithAsteroid` _asspace_shuttle)
  (goto _label))

(fn `DamageApply`
  (params (Damage :type Integer))
  (if (<= (- (`self.HP`) Damage) 0)
    (`ManagerCPP.AddScore` (`self.ManagerCPP`))
    (`GameplayStatics.SpawnEmitterAtLocation` "/Game/StarterContent/Particles/P_Explosion.P_Explosion" (`self.K2_GetActorLocation`))
    (`self.K2_DestroyActor`)
    (else
      (set `self.HP` (- (`self.HP`) Damage)))))

(fn `UserConstructionScript`)