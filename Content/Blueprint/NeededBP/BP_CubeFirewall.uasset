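; BP_CubeFirewall is a cube firewall Blueprint that hands player control to a newly spawned BP_BruCharacter when the Crouch input is pressed.
; The character spawns at the cube's transform, adjusted for collisions but always spawned, and player controller 0 possesses it.
; The cube is not destroyed afterward, and its BeginPlay, overlap and Tick events are disabled stubs.
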(event `InputAction|Crouch`
  (params (Key :type "Key Structure"))
  (:`Pressed`
    (bind _returnvalue (`|SpawnActorFromClass` "/Game/Blueprint/NeededBP/BP_BruCharacter.BP_BruCharacter_C" (`self.GetTransform`) "AdjustIfPossibleButAlwaysSpawn" "OverrideRootScale" null null))
    (`Controller.Possess` (`GameplayStatics.GetPlayerController` 0) _returnvalue)))

(fn `UserConstructionScript`
  (`parent.UserConstructionScript`))