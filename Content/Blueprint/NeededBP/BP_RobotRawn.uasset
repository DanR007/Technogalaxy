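; Possessable robot character that the player takes over by clicking it while outlined, then moves and jumps.
; While possessed, it line-traces each tick to pawns in its sphere, outlining visible ones through InteractiveObjectsInterface and custom depth.
; Crouch spawns a BP_BruCharacter at the robot's transform and calls Possess with no pawn wired.
; Unpossessing snaps the robot to the surface below, and ToStart restores its initial location.
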(event `self.ReceiveBeginPlay`
  (set `self.StartLoc` (`self.K2_GetActorLocation`)))

(event `self.ReceiveTick`
  (params (DeltaSeconds :type "Float (single-precision)"))
  (bind _returnvalue (`GameplayStatics.GetPlayerPawn` 0))
  (for _array_element (`self.OverlappingActors`)
    (if (and (!= _array_element _returnvalue) (== _returnvalue self))
      (bind _outhit (`KismetSystemLibrary.LineTraceSingle` (`self.K2_GetActorLocation`) (`self.K2_GetActorLocation` _array_element) "TraceTypeQuery1"))
      (bind _asinteractive_objects_interface (cast `/Game/Blueprint/InteractiveObjectsInterface` _array_element))
      (`self.ChangeOutline` _asinteractive_objects_interface (== (`.HitActor` (`GameplayStatics.BreakHitResult` _outhit)) _array_element)))))

(event `InputAxis|MoveRight`
  (params (AxisValue :type "Float (single-precision)"))
  (`self.AddMovementInput` (`self.GetActorRightVector`) AxisValue))

(event `self.ChangeOutline`
  (params (isInRange :type Boolean))
  (`PrimitiveComponent.SetRenderCustomDepth` (`self.MainMesh`) isInRange)
  (set `self.isOutline` isInRange))

(event `self.ReceiveActorOnClicked`
  (params (ButtonPressed :type "Key Structure"))
  (if (`self.isOutline`)
    (`Controller.Possess` (`GameplayStatics.GetPlayerController` 0) self)
    (`self.ChangeOutline` false)
    (set `self.isOutline` false)))

(event `self.Sphere.OnComponentBeginOverlap`
  (params (OverlappedComponent :type "PrimitiveComponent Object Reference") (OtherActor :type "Actor Object Reference") (OtherComp :type "PrimitiveComponent Object Reference") (OtherBodyIndex :type Integer) (bFromSweep :type Boolean) (SweepResult :type "HitResult Structure (by ref)"))
  (bind (_aspawn _bsuccess) (cast `Pawn` OtherActor :!pure true))
  (if (and (!= OtherActor self) _bsuccess)
    (`KismetArrayLibrary.Array_AddUnique` (`self.OverlappingActors`) _aspawn)))

(event `self.Sphere.OnComponentEndOverlap`
  (params (OverlappedComponent :type "PrimitiveComponent Object Reference") (OtherActor :type "Actor Object Reference") (OtherComp :type "PrimitiveComponent Object Reference") (OtherBodyIndex :type Integer))
  (bind _asinteractive_objects_interface (cast `/Game/Blueprint/InteractiveObjectsInterface` OtherActor))
  (`self.ChangeOutline` _asinteractive_objects_interface false)
  (bind _aspawn (cast `Pawn` OtherActor))
  (`KismetArrayLibrary.Array_RemoveItem` (`self.OverlappingActors`) _aspawn))

(event `InputAction|Crouch`
  (params (Key :type "Key Structure"))
  (:`Pressed`
    (`|SpawnActorFromClass` "/Game/Blueprint/NeededBP/BP_BruCharacter.BP_BruCharacter_C" (`self.GetTransform`) "AdjustIfPossibleButAlwaysSpawn" "OverrideRootScale" null null)
    (`Controller.Possess` (`GameplayStatics.GetPlayerController` 0) null)))

(event `InputAxis|MoveForward`
  (params (AxisValue :type "Float (single-precision)"))
  (`self.AddMovementInput` (`SceneComponent.GetForwardVector` (`self.Camera`)) AxisValue))

(event `InputAction|Jump`
  (params (Key :type "Key Structure"))
  (:`Pressed`
    (`self.Jump`)))

(event `ToStart`
  (`self.K2_SetActorLocation` (`self.StartLoc`)))

(event `self.ReceiveUnpossessed`
  (params (OldController :type "Controller Object Reference"))
  (bind _returnvalue (`self.K2_GetActorLocation`))
  (bind _outhit (`KismetSystemLibrary.LineTraceSingle` _returnvalue (+ _returnvalue (* (`self.GetActorUpVector`) -2000.0)) "TraceTypeQuery1"))
  (`self.K2_SetActorLocation` (+ (`.Location` (`GameplayStatics.BreakHitResult` _outhit)) (`KismetMathLibrary.MakeVector` 0.0 0.0 (+ (`CapsuleComponent.CapsuleRadius` (`self.CapsuleComponent`)) 2.0)))))

(fn `UserConstructionScript`)