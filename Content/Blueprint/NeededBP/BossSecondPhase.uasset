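; BossSecondPhase is an actor that runs a boss's second phase by spawning hazard zones and serving as the game's completion trigger.
; A looping timer started on BeginPlay calls SpawnRedZones, which repeatedly spawns a BackZoneTemp actor at the boss's own transform.
; When the player's capsule overlaps the Box, it marks the game complete on the cached ProgressActor and opens the ComicsFinal level.
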(event `self.ReceiveBeginPlay`
  (`parent.ReceiveBeginPlay`)
  (`KismetSystemLibrary.K2_SetTimer` self "SpawnRedZones" 5.0 true 1.0)
  (bind _returnvalue (`GameplayStatics.GetActorOfClass` "/Script/ROBOTERRAbackstory.ProgressActor"))
  (set `self.ProgressActor` _returnvalue))

(event `self.Box.OnComponentBeginOverlap`
  (params (OverlappedComponent :type "PrimitiveComponent Object Reference") (OtherActor :type "Actor Object Reference") (OtherComp :type "PrimitiveComponent Object Reference") (OtherBodyIndex :type Integer) (bFromSweep :type Boolean) (SweepResult :type "HitResult Structure (by ref)"))
  (if (and (== OtherActor (`GameplayStatics.GetPlayerCharacter` 0)) (`.bSuccess` (cast `CapsuleComponent` OtherComp :!pure true)))
    (`ProgressActor.SetGameComplete` (`self.ProgressActor`))
    (`GameplayStatics.OpenLevelBySoftObjectPtr` "/Game/Levels/ComicsFinal.ComicsFinal")))

(fn `SpawnRedZones`
  (`|SpawnActorFromClass` "/Game/Blueprint/NeededBP/BackZoneTemp.BackZoneTemp_C" (`self.GetTransform`) "AlwaysSpawn" "OverrideRootScale" null null))

(fn `UserConstructionScript`
  (`parent.UserConstructionScript`))