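; ExtraJumpActor is a possessable alternate character that moves along the camera's forward vector and can jump.
; Pressing Crouch or overlapping a Barrier with the capsule spawns a new BP_BruCharacter at its current transform and hands player 0's controller to it.
; When unpossessed, it teleports back to the location stored at BeginPlay, leaving the new character where the switch happened.
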(event `self.CapsuleComponent.OnComponentBeginOverlap`
  (params (OverlappedComponent :type "PrimitiveComponent Object Reference") (OtherActor :type "Actor Object Reference") (OtherComp :type "PrimitiveComponent Object Reference") (OtherBodyIndex :type Integer) (bFromSweep :type Boolean) (SweepResult :type "HitResult Structure (by ref)"))
  (cast `/Game/Blueprint/NeededBP/Barrier` OtherActor)
  (bind _returnvalue (`|SpawnActorFromClass` "/Game/Blueprint/NeededBP/BP_BruCharacter.BP_BruCharacter_C" (`self.GetTransform`) "AdjustIfPossibleButAlwaysSpawn" "OverrideRootScale" null null :!label _label))
  (`Controller.Possess` (`GameplayStatics.GetPlayerController` 0) _returnvalue))

(event `InputAction|Crouch`
  (params (Key :type "Key Structure"))
  (:`Pressed`
    (goto _label)))

(event `self.ReceiveUnpossessed`
  (params (OldController :type "Controller Object Reference"))
  (`self.K2_SetActorLocation` (`self.startLoc`)))

(event `InputAxis|MoveForward`
  (params (AxisValue :type "Float (single-precision)"))
  (`self.AddMovementInput` (`SceneComponent.GetForwardVector` (`self.Camera`)) AxisValue))

(event `InputAction|Jump`
  (params (Key :type "Key Structure"))
  (:`Pressed`
    (`self.Jump`)))

(event `self.ReceiveBeginPlay`
  (`parent.ReceiveBeginPlay`)
  (set `self.startLoc` (`self.K2_GetActorLocation`)))

(fn `UserConstructionScript`
  (`parent.UserConstructionScript`))