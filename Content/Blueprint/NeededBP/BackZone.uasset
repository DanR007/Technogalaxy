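; BackZone is a trigger box that switches the player from their current pawn into a newly spawned BP_BruCharacter.
; When the player character's capsule overlaps the Box, it spawns that character at SaveActor's location with the overlapping actor's rotation and scale, then possesses it.
; If the overlapping actor is a BP_RobotRawn, it then calls ToStart on it.
; Other overlaps only print a debug string.
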(event `self.Box.OnComponentBeginOverlap`
  (params (OverlappedComponent :type "PrimitiveComponent Object Reference") (OtherActor :type "Actor Object Reference") (OtherComp :type "PrimitiveComponent Object Reference") (OtherBodyIndex :type Integer) (bFromSweep :type Boolean) (SweepResult :type "HitResult Structure (by ref)"))
  (bind (_returnvalue_location _returnvalue_rotation _returnvalue_scale) (`KismetMathLibrary.BreakTransform` (`self.GetTransform` OtherActor)))
  (if (and (`.bSuccess` (cast `CapsuleComponent` OtherComp :!pure true)) (== OtherActor (`GameplayStatics.GetPlayerCharacter` 0)))
    (bind _returnvalue (`|SpawnActorFromClass` "/Game/Blueprint/NeededBP/BP_BruCharacter.BP_BruCharacter_C" (`KismetMathLibrary.MakeTransform` (`self.K2_GetActorLocation` (`self.saveActor`)) _returnvalue_rotation _returnvalue_scale) "AdjustIfPossibleButAlwaysSpawn" "OverrideRootScale" null null))
    (`Controller.Possess` (`GameplayStatics.GetPlayerController` 0) _returnvalue)
    (bind _asbp_robot_rawn (cast `/Game/Blueprint/NeededBP/BP_RobotRawn` OtherActor))
    (`/Game/Blueprint/NeededBP/BP_RobotRawn.ToStart` _asbp_robot_rawn)
    (else
      (`KismetSystemLibrary.PrintString` "Hello"))))

(fn `UserConstructionScript`)