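; BPShuttleCPP is an enemy shuttle that flies steadily and fires bullets on a repeating timer.
; BeginPlay starts a looping Shoot timer with an interval of SpeedRel plus a random offset, and caches the level's ManagerCPP actor.
; Shoot spawns an EnemyBullet at the shuttle's transform.
; Tick moves it opposite its forward vector by Speed each frame, without sweep or delta-time scaling.
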(event `self.ReceiveBeginPlay`
  (`KismetSystemLibrary.K2_SetTimer` null "Shoot" (+ (`self.speedRel`) (`KismetMathLibrary.RandomFloatInRange` 0.0 3.0)) true)
  (bind _returnvalue (`GameplayStatics.GetActorOfClass` "/Script/ROBOTERRAbackstory.ManagerCPP"))
  (set `self.ManagerCPP` _returnvalue))

(event `self.ReceiveTick`
  (params (DeltaSeconds :type "Float (single-precision)"))
  (`self.K2_AddActorWorldOffset` (* (`self.GetActorForwardVector`) (* (`self.speed`) -1.0))))

(fn `Shoot`
  (`|SpawnActorFromClass` "/Game/Blueprint/NeededBP/EnemyBullet.EnemyBullet_C" (`self.GetTransform`) "AlwaysSpawn" "OverrideRootScale" null null))

(fn `UserConstructionScript`)