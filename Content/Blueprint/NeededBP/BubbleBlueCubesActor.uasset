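; BubbleBlueCubesActor is a trigger actor that periodically raises a NotUnderstand flag, apparently for a hint bubble, after the player has entered its box.
; The box overlap stores the player character, which is never cleared here, so Tick keeps the cycle running.
; Latent delays in Tick pace it: after a wait, NotUnderstand turns on briefly unless Understand is set.
; Nothing in this graph sets Understand or reads NotUnderstand.
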(event `self.ReceiveTick`
  (params (DeltaSeconds :type "Float (single-precision)"))
  (`/Engine/EditorBlueprintResources/StandardMacros.IsValid` (`self.Player`)
    (:`Is Valid`
      (`KismetSystemLibrary.Delay` 10.0)
      (if (not (`self.Understand`))
        (set `self.NotUnderstand` true)
        (`KismetSystemLibrary.Delay` 5.0)
        (set `self.NotUnderstand` false)))))

(event `self.Box.OnComponentBeginOverlap`
  (params (OverlappedComponent :type "PrimitiveComponent Object Reference") (OtherActor :type "Actor Object Reference") (OtherComp :type "PrimitiveComponent Object Reference") (OtherBodyIndex :type Integer) (bFromSweep :type Boolean) (SweepResult :type "HitResult Structure (by ref)"))
  (if (== OtherActor (`GameplayStatics.GetPlayerCharacter` 0))
    (set `self.Player` (cast `Character` OtherActor :!pure true))))

(fn `UserConstructionScript`)