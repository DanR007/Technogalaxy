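; BoostDoubleJump is a pickup actor that raises a BP_BruCharacter's jump height on overlap with its Sphere.
; Overlap multiplies the character's JumpZVelocity by 1.4, disables Sphere collision and hides the Arrow.
; After a ten-second delay it multiplies the velocity again by 1.2 instead of restoring it.
; Sphere collision returns as query-only, but the Arrow stays hidden because the second call also hides it.
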(event `self.Sphere.OnComponentBeginOverlap`
  (params (OverlappedComponent :type "PrimitiveComponent Object Reference") (OtherActor :type "Actor Object Reference") (OtherComp :type "PrimitiveComponent Object Reference") (OtherBodyIndex :type Integer) (bFromSweep :type Boolean) (SweepResult :type "HitResult Structure (by ref)"))
  (bind _asbp_bru_character (cast `/Game/Blueprint/BP_BruCharacter` OtherActor))
  (bind _charactermovement (`Character.CharacterMovement` _asbp_bru_character))
  (set `CharacterMovementComponent.JumpZVelocity` (* (`CharacterMovementComponent.JumpZVelocity` _charactermovement) 1.4) _charactermovement)
  (`PrimitiveComponent.SetCollisionEnabled` (`self.Sphere`) "NoCollision")
  (`SceneComponent.SetHiddenInGame` (`self.Arrow`) true false)
  (`KismetSystemLibrary.Delay` 10.0)
  (bind _charactermovement_2 (`Character.CharacterMovement` _asbp_bru_character))
  (set `CharacterMovementComponent.JumpZVelocity` (* (`CharacterMovementComponent.JumpZVelocity` _charactermovement_2) 1.2) _charactermovement_2)
  (`PrimitiveComponent.SetCollisionEnabled` (`self.Sphere`) "QueryOnly")
  (`SceneComponent.SetHiddenInGame` (`self.Arrow`) true false))

(fn `UserConstructionScript`)