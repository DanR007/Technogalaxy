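; PowerUp is a pickup actor that raises the Power of a SpaceShuttle that touches it.
; It drifts backward along its forward axis by a fixed step every tick, independent of delta time.
; Sphere overlap with a shuttle adds one Power, clamped to MaxPower from the ManagerCPP actor found at BeginPlay, then destroys the pickup.
; Overlapping a BlockingVolume also destroys it.
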(event `self.ReceiveBeginPlay`
  (bind _returnvalue (`GameplayStatics.GetActorOfClass` "/Script/ROBOTERRAbackstory.ManagerCPP"))
  (set `self.ManagerCpp` _returnvalue))

(event `self.ReceiveActorBeginOverlap`
  (params (OtherActor :type "Actor Object Reference"))
  (cast `BlockingVolume` OtherActor)
  (`self.K2_DestroyActor`))

(event `self.ReceiveTick`
  (params (DeltaSeconds :type "Float (single-precision)"))
  (`self.K2_AddActorWorldOffset` (* (`self.GetActorForwardVector`) -1.5)))

(event `self.Sphere.OnComponentBeginOverlap`
  (params (OverlappedComponent :type "PrimitiveComponent Object Reference") (OtherActor :type "Actor Object Reference") (OtherComp :type "PrimitiveComponent Object Reference") (OtherBodyIndex :type Integer) (bFromSweep :type Boolean) (SweepResult :type "HitResult Structure (by ref)"))
  (bind _asspace_shuttle (cast `/Game/Blueprint/NeededBP/SpaceShuttle` OtherActor))
  (set `/Game/Blueprint/NeededBP/SpaceShuttle.Power` (`KismetMathLibrary.Clamp` (+ (`/Game/Blueprint/NeededBP/SpaceShuttle.Power` _asspace_shuttle) 1) 0 (`ManagerCPP.maxPower` (`self.ManagerCpp`))) _asspace_shuttle)
  (`self.K2_DestroyActor`))

(fn `UserConstructionScript`)