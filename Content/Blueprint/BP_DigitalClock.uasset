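; BP_DigitalClock is a possessable clock whose time the player sets with the MoveRight axis.
; Clicking its MainMesh makes player controller 0 possess it.
; Axis input passes through a short Delay that throttles changes to Minutes, which roll over at 60 and increment Hour.
; Hour clamps at 23 instead of wrapping, minutes cannot borrow backwards, and these graphs contain no display update.
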(event `self.MainMesh.OnClicked`
  (params (TouchedComponent :type "PrimitiveComponent Object Reference") (ButtonPressed :type "Key Structure"))
  (`Controller.Possess` (`GameplayStatics.GetPlayerController` 0) self))

(event `InputAxis|MoveRight`
  (params (AxisValue :type "Float (single-precision)"))
  (`KismetSystemLibrary.Delay` 0.1)
  (bind _output_get (set `self.minutes` (`KismetMathLibrary.Clamp` (`KismetMathLibrary.FTrunc` (+ AxisValue (`KismetMathLibrary.Conv_IntToDouble` (`self.minutes`)))) 0 60)))
  (if (>= _output_get 60)
    (set `self.minutes` 0)
    (bind _result (`/Engine/EditorBlueprintResources/StandardMacros.IncrementInt` (`self.hour`))
      (:`  `
        (set `self.hour` (`KismetMathLibrary.Clamp` _result 0 23))))))

(fn `UserConstructionScript`
  (`parent.UserConstructionScript`))