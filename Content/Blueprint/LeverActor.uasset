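; Clickable lever actor that toggles a linked door, usable only while its range-driven outline is on.
; ChangeOutline sets custom depth on both meshes for the highlight and gates clicks on either mesh.
; Each click flips the state and plays or reverses a timeline that pitches the Pivot.
; When the timeline finishes, it passes the current state to LinkedDoor through ButtonChangePressed.
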(event `self.MainMesh.OnClicked`
  (params (TouchedComponent :type "PrimitiveComponent Object Reference") (ButtonPressed :type "Key Structure"))
  (if (`self.isOutline`) :!label _label
    (bind _output_get (set `self.isClicked` (not (`self.isClicked`))))
    (if _output_get
      (bind (_direction _newtrack_0) (`Timeline|TurnOffOrOn` :!label _label_2)
        (:`Update`
          (`SceneComponent.K2_SetRelativeRotation` (`self.Pivot`) (`KismetMathLibrary.MakeRotator` 0.0 _newtrack_0) false false))
        (:`Finished`
          (`/Game/Blueprint/LinkedWithTheButton.ButtonChangePressed` (`self.LinkedDoor`) (`self.isClicked`))))
      (else
        (goto _label_2 :!via `Reverse`)))))

(event `self.LeverMesh.OnClicked`
  (params (TouchedComponent :type "PrimitiveComponent Object Reference") (ButtonPressed :type "Key Structure"))
  (goto _label))

(event `/Game/Blueprint/InteractiveObjectsInterface.ChangeOutline`
  (params (isInRange :type Boolean))
  (`PrimitiveComponent.SetRenderCustomDepth` (`self.MainMesh`) isInRange)
  (`PrimitiveComponent.SetRenderCustomDepth` (`self.LeverMesh`) isInRange)
  (set `self.isOutline` isInRange))

(fn `UserConstructionScript`)