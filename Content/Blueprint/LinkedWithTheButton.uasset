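; Button-linked actor that moves between StartLocation and EndLocation when its ButtonChangePressed event updates the pressed state.
; In loop mode, Tick drives Timeline_0 while working, flipping direction after a short delay at each end to ping-pong the actor.
; Otherwise OpenOnce plays on press and reverses from its end on release, with OnceOk tracking whether it finished opening.
; Both timelines feed a location lerp without sweep.
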(event `self.ReceiveTick`
  (params (DeltaSeconds :type "Float (single-precision)"))
  (if (and (`self.isLoop`) (`self.isWorking`))
    (if (not (`self.onEnd`))
      (bind (_direction _newtrack_0) (`Timeline|Timeline_0` :!label _label)
        (:`Update`
          (`self.K2_SetActorLocation` (`KismetMathLibrary.VLerp` (`self.StartLocation`) (`self.EndLocation`) _newtrack_0)))
        (:`Finished`
          (`KismetSystemLibrary.Delay` 2.0)
          (set `self.onEnd` (not (`self.onEnd`)))))
      (else
        (goto _label :!via `Reverse`)))))

(event `ButtonChangePressed`
  (params (isPressed :type Boolean))
  (bind _output_get (set `self.isWorking` isPressed))
  (if (not (`self.isLoop`))
    (if (not (`self.OnceOk`))
      (if _output_get
        (bind (_direction _newtrack_0) (`Timeline|OpenOnce` :!label _label_2)
          (:`Update`
            (`self.K2_SetActorLocation` (`KismetMathLibrary.VLerp` (`self.StartLocation`) (`self.EndLocation`) _newtrack_0)))
          (:`Finished`
            (set `self.OnceOk` _output_get)))
        (else
          (goto _label_2 :!via `ReverseFromEnd`)))
      (else
        (goto _label_2 :!via `ReverseFromEnd`)))))

(fn `UserConstructionScript`)