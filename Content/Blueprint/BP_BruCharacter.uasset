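; BP_BruCharacter is a character that the player can switch control to by clicking it while it is outlined.
; A collider tracks nearby pawns, and on Tick the possessed character line-traces to each, toggling its outline through InteractiveObjectsInterface based on visibility.
; The outline uses mesh custom depth and gates the click that makes the player controller possess that character.
; Possession also enables the mouse cursor and click events.
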(event `self.ReceivePossessed`
  (params (NewController :type "Controller Object Reference"))
  (bind _returnvalue (`GameplayStatics.GetPlayerController` 0))
  (set `PlayerController.bShowMouseCursor` true _returnvalue)
  (set `PlayerController.bEnableClickEvents` true _returnvalue))

(event `self.ReceiveTick`
  (params (DeltaSeconds :type "Float (single-precision)"))
  (bind _returnvalue (`GameplayStatics.GetPlayerPawn` 0))
  (for _array_element (`self.OverlappingActors`)
    (if (and (!= _array_element _returnvalue) (== _returnvalue self))
      (bind _outhit (`KismetSystemLibrary.LineTraceSingle` (`self.K2_GetActorLocation`) (`self.K2_GetActorLocation` _array_element) "TraceTypeQuery1"))
      (bind _asinteractive_objects_interface (cast `/Game/Blueprint/InteractiveObjectsInterface` _array_element))
      (`self.ChangeOutline` _asinteractive_objects_interface (== (`.HitActor` (`GameplayStatics.BreakHitResult` _outhit)) _array_element)))))

(event `self.ColliderOfObject.OnComponentBeginOverlap`
  (params (OverlappedComponent :type "PrimitiveComponent Object Reference") (OtherActor :type "Actor Object Reference") (OtherComp :type "PrimitiveComponent Object Reference") (OtherBodyIndex :type Integer) (bFromSweep :type Boolean) (SweepResult :type "HitResult Structure (by ref)"))
  (bind (_aspawn _bsuccess) (cast `Pawn` OtherActor :!pure true))
  (if (and (!= OtherActor self) _bsuccess)
    (`KismetArrayLibrary.Array_AddUnique` (`self.OverlappingActors`) _aspawn)))

(event `self.ColliderOfObject.OnComponentEndOverlap`
  (params (OverlappedComponent :type "PrimitiveComponent Object Reference") (OtherActor :type "Actor Object Reference") (OtherComp :type "PrimitiveComponent Object Reference") (OtherBodyIndex :type Integer))
  (bind _asinteractive_objects_interface (cast `/Game/Blueprint/InteractiveObjectsInterface` OtherActor))
  (`self.ChangeOutline` _asinteractive_objects_interface false)
  (bind _aspawn (cast `Pawn` OtherActor))
  (`KismetArrayLibrary.Array_RemoveItem` (`self.OverlappingActors`) _aspawn))

(event `self.ChangeOutline`
  (params (isInRange :type Boolean))
  (`PrimitiveComponent.SetRenderCustomDepth` (`self.Mesh`) isInRange)
  (set `self.isOutline` isInRange))

(event `self.ReceiveActorOnClicked`
  (params (ButtonPressed :type "Key Structure"))
  (if (`self.isOutline`)
    (`Controller.Possess` (`GameplayStatics.GetPlayerController` 0) self)
    (`self.ChangeOutline` false)
    (set `self.isOutline` false)))

(fn `UserConstructionScript`)